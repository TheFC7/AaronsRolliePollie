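; Level 1 floating island prop Blueprint that moves its static mesh along a spline as a moving platform.
; On BeginPlay a timeline plays, and its track value, scaled by the spline length, sets the mesh's world location along the spline each update.
; An older sine-based oscillation around a saved start position remains in the graph but is disconnected, and Tick is empty.
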(event EventTick
  (params (DeltaSeconds :type Float%20%28single-precision%29))
  ;[1 1 1] Sin Controller, creates variables between platforms
)

(event EventBeginPlay
  ;[1 1 1] Spline BP
  (bind _sidetosdie (Timeline|MovePlatfrom Play)
    (:Update
      (Transformation|SetWorldLocation (Variables|Default|GetStaticMesh) (Spline|GetLocationatDistanceAlongSpline (Variables|Default|GetSpline) (* _sidetosdie (Spline|GetSplineLength (Variables|Default|GetSpline))) "World") false false))))

(fn ConstructionScript)